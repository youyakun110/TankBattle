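; MoTar_BP is a mortar Blueprint that sets up its aiming and health bar when play begins.
; On BeginPlay it initialises the TankAiming component with the TankBarrel and the MotarDome turret.
; It then passes itself to the HealthBar widget as MyTank, so it reuses tank aiming and health bar parts.
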(event `self.ReceiveBeginPlay`
  (`TankAimingComponent.Initialise` (`self.TankAiming`) (`self.TankBarrel`) (`self.Motar_Dome`))
  (`self.Initialise`))

(fn `Initialise`
  (bind _ashealth_bar (cast `/Game/UIWidgets/HealthBar` (`WidgetComponent.GetUserWidgetObject` (`self.HealthBar`))))
  (set `/Game/UIWidgets/HealthBar.MyTank` self _ashealth_bar))

(fn `UserConstructionScript`)